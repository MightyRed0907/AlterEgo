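; BP_Cell is one cell in a grid display: each tick it samples the pixel color at its X/Y from the AlterEgo player controller.
; When the color changes noticeably, its mode decides the response: tint a dynamic material, roll the mesh by brightness, or morph.
; Morphing steps one mesh at a time through a set toward a brightness-based index.
; Functions switch modes, cycle each mode's mesh assets and adjust scale within limits.
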(event Custom|SetColoring
  (Rendering|Material|SetVectorParameterValue (Variables|Default|GetMaterialInstance) "Color" (Variables|Default|GetColor) :!class /Script/Engine.MaterialInstanceDynamic))

(event Custom|SetRotating
  (Transformation|SetWorldRotation (Variables|Default|GetMesh) (CallFunction|CalculateRotation) false false))

(event Custom|ChangeMode
  (params (NewMode :type CellMode%20Enum :default "NewEnumerator0"))
  (bind _mesh (Variables|Default|GetMesh))
  (bind _mesh_2 (Variables|Default|GetMesh))
  (bind _mesh_3 (Variables|Default|GetMesh))
  (bind _output_get (Variables|Default|SetCellMode NewMode))
  (switch Utilities|FlowControl|Switch|SwitchonCellMode _output_get
    (:NewEnumerator0
      (Variables|MeshAsset|SetColoringAssetIndex 0)
      (Components|StaticMesh|SetStaticMesh _mesh_2 (.mesh (Utilities|Array|Get(acopy) (Variables|MeshAsset|GetColoringAssets) (Variables|MeshAsset|GetColoringAssetIndex))))
      (Transformation|SetRelativeTransform _mesh_2 (.transform (Utilities|Array|Get(acopy) (Variables|MeshAsset|GetColoringAssets) (Variables|MeshAsset|GetColoringAssetIndex))) false false)
      (bind _returnvalue (Rendering|Material|CreateDynamicMaterialInstance (Variables|Default|GetMesh) 0 "/Game/AlterEgo/Materials/M_Cell.M_Cell" "None" :!class /Script/Engine.PrimitiveComponent))
      (bind _output_get_2 (Variables|Default|SetMaterialInstance _returnvalue))
      (Rendering|Material|SetVectorParameterValue _output_get_2 "Color" (Variables|Default|GetColor) :!class /Script/Engine.MaterialInstanceDynamic))
    (:NewEnumerator1
      (Variables|MeshAsset|SetRotatingAssetIndex 0)
      (Components|StaticMesh|SetStaticMesh _mesh_3 (.mesh (Utilities|Array|Get(acopy) (Variables|MeshAsset|GetRotatingAssets) (Variables|MeshAsset|GetRotatingAssetIndex))))
      (Transformation|SetRelativeTransform _mesh_3 (.transform (Utilities|Array|Get(acopy) (Variables|MeshAsset|GetRotatingAssets) (Variables|MeshAsset|GetRotatingAssetIndex))) false false)
      (Rendering|Material|SetMaterial (Variables|Default|GetMesh) 0 "/Engine/MapTemplates/Sky/Desert_Outer_HDR_Mat.Desert_Outer_HDR_Mat"))
    (:NewEnumerator3
      (Variables|MeshAsset|SetMorphingAssetIndex 0)
      (Variables|MeshAsset|SetMorphingAssetMeshIndex 0)
      (Components|StaticMesh|SetStaticMesh _mesh (.mesh (Utilities|Array|Get(acopy) (.cellassets (Utilities|Array|Get(acopy) (Variables|MeshAsset|GetMorphingAssets) (Variables|MeshAsset|GetRotatingAssetIndex))) (Variables|MeshAsset|GetMorphingAssetMeshIndex))))
      (Transformation|SetRelativeTransform _mesh (.transform (Utilities|Array|Get(acopy) (.cellassets (Utilities|Array|Get(acopy) (Variables|MeshAsset|GetMorphingAssets) (Variables|MeshAsset|GetRotatingAssetIndex))) (Variables|MeshAsset|GetMorphingAssetMeshIndex))) false false)
      (Rendering|Material|SetMaterial (Variables|Default|GetMesh) 0 "/Game/AlterEgo/Materials/M_Morphing.M_Morphing"))))

(event Custom|SetMorphing
  (bind _mesh (Variables|Default|GetMesh))
  (bind _morphingassets (Variables|MeshAsset|GetMorphingAssets))
  (bind _morphingassetindex (Variables|MeshAsset|GetMorphingAssetIndex))
  (bind _morphingassetmeshindex (Variables|MeshAsset|GetMorphingAssetMeshIndex))
  (bind _output (Utilities|Array|Get(acopy) _morphingassets _morphingassetindex))
  (bind _output_2 (Utilities|Array|Get(acopy) (.cellassets _output) _morphingassetmeshindex))
  (CallFunction|CalcuateMorphing)
  (Components|StaticMesh|SetStaticMesh _mesh (.mesh _output_2))
  (Transformation|SetRelativeTransform _mesh (.transform _output_2) false false))

(event EventBeginPlay
  (Variables|Default|SetPC_Ref (.AsBPPC%20Alter%20Ego (Utilities|Casting|CastToBPPC_AlterEgo (Game|GetPlayerController 0))))
  (CallFunction|ChangeMode "NewEnumerator0"))

(event EventTick
  (params (DeltaSeconds :type Float%20%28single-precision%29))
  (Variables|Default|SetNewColor (Default|GetPixelColor (Variables|Default|GetPC_Ref) (Variables|Default|GetX) (Variables|Default|GetY)))
  (if (CallFunction|IsColorChanged)
    (Variables|Default|SetColor (Variables|Default|GetNewColor))
    (switch Utilities|FlowControl|Switch|SwitchonCellMode (Variables|Default|GetCellMode)
      (:NewEnumerator0
        (CallFunction|SetColoring))
      (:NewEnumerator1
        (CallFunction|SetRotating))
      (:NewEnumerator3
        (CallFunction|SetMorphing)))))

(fn ConstructionScript
  (bind _returnvalue (Rendering|Material|CreateDynamicMaterialInstance (Variables|Default|GetMesh) 0 0 "None" :!class /Script/Engine.PrimitiveComponent))
  (Rendering|Material|SetVectorParameterValue _returnvalue "Color" (Variables|Default|GetColor) :!class /Script/Engine.MaterialInstanceDynamic))

(fn IsBlack
  (bind _color (Variables|Default|GetColor))
  (return (Math|Boolean|ANDBoolean (< (.r _color) 0.03) (< (.g _color) 0.03) (< (.b _color) 0.03))))

(fn IsColorChanged
  (return (> (Class|KismetMathLibrary|LinearColorDistance (Variables|Default|GetColor) (Variables|Default|GetNewColor)) 0.1)))

(fn LoadNextMesh
  (bind _mesh (Variables|Default|GetMesh))
  (bind _mesh_2 (Variables|Default|GetMesh))
  (bind _mesh_3 (Variables|Default|GetMesh))
  (switch Utilities|FlowControl|Switch|SwitchonCellMode (Variables|Default|GetCellMode)
    (:NewEnumerator0
      (Variables|MeshAsset|SetColoringAssetIndex (Math|Integer|%(Integer) (+ (Variables|MeshAsset|GetColoringAssetIndex) 1) (Utilities|Array|Length (Variables|MeshAsset|GetColoringAssets))))
      (Components|StaticMesh|SetStaticMesh _mesh_3 (.mesh (Utilities|Array|Get(acopy) (Variables|MeshAsset|GetColoringAssets) (Variables|MeshAsset|GetColoringAssetIndex))))
      (Transformation|SetRelativeTransform _mesh_3 (.transform (Utilities|Array|Get(acopy) (Variables|MeshAsset|GetColoringAssets) (Variables|MeshAsset|GetColoringAssetIndex))) false false)
      (bind _returnvalue (Rendering|Material|CreateDynamicMaterialInstance (Variables|Default|GetMesh) 0 0 "None" :!class /Script/Engine.PrimitiveComponent))
      (bind _output_get (Variables|Default|SetMaterialInstance _returnvalue))
      (Rendering|Material|SetVectorParameterValue _output_get "Color" (Variables|Default|GetColor) :!class /Script/Engine.MaterialInstanceDynamic))
    (:NewEnumerator1
      (Variables|MeshAsset|SetRotatingAssetIndex (Math|Integer|%(Integer) (+ (Variables|MeshAsset|GetRotatingAssetIndex) 1) (Utilities|Array|Length (Variables|MeshAsset|GetRotatingAssets))))
      (Components|StaticMesh|SetStaticMesh _mesh_2 (.mesh (Utilities|Array|Get(acopy) (Variables|MeshAsset|GetRotatingAssets) (Variables|MeshAsset|GetRotatingAssetIndex))))
      (Transformation|SetRelativeTransform _mesh_2 (.transform (Utilities|Array|Get(acopy) (Variables|MeshAsset|GetRotatingAssets) (Variables|MeshAsset|GetRotatingAssetIndex))) false false))
    (:NewEnumerator3
      (Variables|MeshAsset|SetMorphingAssetIndex (Math|Integer|%(Integer) (+ (Variables|MeshAsset|GetMorphingAssetIndex) 1) (Utilities|Array|Length (Variables|MeshAsset|GetMorphingAssets))))
      (Variables|MeshAsset|SetMorphingAssetMeshIndex 0)
      (Components|StaticMesh|SetStaticMesh _mesh (.mesh (Utilities|Array|Get(acopy) (.cellassets (Utilities|Array|Get(acopy) (Variables|MeshAsset|GetMorphingAssets) (Variables|MeshAsset|GetRotatingAssetIndex))) (Variables|MeshAsset|GetMorphingAssetMeshIndex))))
      (Transformation|SetRelativeTransform _mesh (.transform (Utilities|Array|Get(acopy) (.cellassets (Utilities|Array|Get(acopy) (Variables|MeshAsset|GetMorphingAssets) (Variables|MeshAsset|GetRotatingAssetIndex))) (Variables|MeshAsset|GetMorphingAssetMeshIndex))) false false))))

(fn ScaleSize
  (params (Increase :type Boolean))
  (if Increase
    (LocalVariables|SetDelta 0.1)
    (else
      (LocalVariables|SetDelta -0.1)))
  (LocalVariables|SetNewScale (Math|Float|Clamp(Float) (+ (LocalVariables|GetDelta) (.x (Variables|/Script/Engine.SceneComponent|GetRelativeScale3D (Variables|Default|GetMesh)))) 0.5 1.5))
  (Transformation|SetRelativeScale3D (Variables|Default|GetMesh) (Math|Vector|MakeVector (LocalVariables|GetNewScale) (LocalVariables|GetNewScale) (LocalVariables|GetNewScale))))

(fn CalculateRotation
  (bind _color (Variables|Default|GetColor))
  (return (Math|Rotator|MakeRotator (* (/ (+ (.r _color) (.g _color) (.b _color)) 3.0) 1.8e+02) 0.0 0.0)))

(fn CalcuateMorphing
  (bind _color (Variables|Default|GetColor))
  (bind _morphingassets (Variables|MeshAsset|GetMorphingAssets))
  (bind _morphingassetmeshindex (Variables|MeshAsset|GetMorphingAssetMeshIndex))
  (bind _morphingassetindex (Variables|MeshAsset|GetMorphingAssetIndex))
  (bind _output (Utilities|Array|Get(acopy) _morphingassets _morphingassetindex))
  (bind _returnvalue (Utilities|Array|Length (.cellassets _output)))
  (LocalVariables|SetBright (+ (.r _color) (.g _color) (.b _color)))
  (LocalVariables|SetNewIndex (Math|Integer|Clamp(Integer) (- (Math|Float|Truncate (/ (LocalVariables|GetBright) (/ 2.0 (Math|Conversions|ToFloat(Integer) _returnvalue)))) 1) 0 (- _returnvalue 1)))
  (if (< (Variables|MeshAsset|GetMorphingAssetMeshIndex) (LocalVariables|GetNewIndex))
    (Math|Integer|IncrementInt _morphingassetmeshindex
      (:%20%20
        (Development|PrintString (Utilities|String|ToString(Integer) (Variables|MeshAsset|GetMorphingAssetMeshIndex)) :!label _label)))
    (elif (> (Variables|MeshAsset|GetMorphingAssetMeshIndex) (LocalVariables|GetNewIndex))
      (Math|Integer|DecrementInt _morphingassetmeshindex
        (:%20%20
          (goto _label))))))
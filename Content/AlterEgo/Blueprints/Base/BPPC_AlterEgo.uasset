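; Player controller for AlterEgo that turns a live webcam feed into a grid of BP_Cell actors.
; On start it lowers graphics settings and lists cameras, then opens one through Media Player and spawns cells sized to the frame.
; Each Tick draws the video to a render target and caches raw pixels, exposed through GetPixelColor.
; Input cycles cameras, cell meshes and Coloring/Rotating/Morphing modes, and controls cell size, screen percentage, movement, zoom and UI.
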(event Custom|GetAllCameras
  ;[0 0.4441 1] Get all webcam connected
  (bind _outdevices (Class|MediaBlueprintFunctionLibrary|EnumerateVideoCaptureDevices -1))
  (Variables|Devices|SetConnectedCameras _outdevices)
  (bind _outdevices_2 (Class|MediaBlueprintFunctionLibrary|EnumerateWebcamCaptureDevices -1))
  (for _array_element _outdevices_2
    (Utilities|Array|AddUnique (Variables|Devices|GetConnectedCameras) _array_element))
  (Variables|Devices|SetConnectedCameraId 0)
  (Default|AddLogText (Variables|Default|GetMainHUD_Ref) (Utilities|Text|FormatText "{num} cameras connected!" (Utilities|Array|Length (Variables|Devices|GetConnectedCameras))) "(R=0.000000,G=0.570285,B=1.000000,A=1.000000)"))

(event Custom|GetTextureRenderAndSpawnCells
  ;[0 1 0.7159] Setup Texture Render and spawn cells
  (bind (_canvas _size _context) (Rendering|BeginDrawCanvastoRenderTarget (Variables|MediaPlayer|GetTextureRender) :!label _label))
  (Utilities|IsValid _canvas
    (:Is%20Valid
      (Canvas|DrawTexture :self _canvas :RenderTexture "/Game/AlterEgo/Movies/MediaPlayer_Video.MediaPlayer_Video" :ScreenSize (Math|Vector2D|MakeVector2D (Math|Conversions|ToFloat(Integer) (Variables|MediaPlayer|GetWidth)) (Math|Conversions|ToFloat(Integer) (Variables|MediaPlayer|GetHeight))) :CoordinateSize "(X=1.000000,Y=1.000000)" :PivotPoint "(X=0.500000,Y=0.500000)")
      (Rendering|EndDrawCanvastoRenderTarget _context)
      (CallFunction|SpawnCells))
    (:Is%20Not%20Valid
      (Utilities|FlowControl|Delay 1.0)
      (goto _label))))

(event Custom|RetrySpawnCells
  ;[1 0 0.0186] Control
  (CallFunction|ConnectDevice)
  (CallFunction|GetTextureRenderandSpawnCells))

(event Custom|GraphicSetting
  ;[0 1 0.1169] Graphic Setting
  (Development|ExecuteConsoleCommand "r.ViewDistanceScale = 0.1" 0)
  (Development|ExecuteConsoleCommand "sg.PostProcessQuality = 0" 0)
  (Development|ExecuteConsoleCommand "sg.ShadowQuality = 0" 0)
  (Development|ExecuteConsoleCommand "sg.TextureQuality = 0" 0)
  (Development|ExecuteConsoleCommand "sg.EffectsQuality = 0" 0)
  (Development|ExecuteConsoleCommand "r.DetailMode = 0" 0))

(event Custom|ConnectDevice
  ;[0.3042 0 1] Connect the next webcam and initialize Texture Render
  (Utilities|FlowControl|Sequence
    (:then_0
      (bind _returnvalue (Class|MediaPlayer|OpenUrl (Variables|MediaPlayer|GetMediaPlayer) (.url (Utilities|Array|Get(acopy) (Variables|Devices|GetConnectedCameras) (Variables|Devices|GetConnectedCameraId)))))
      (Utilities|FlowControl|Delay 2.5)
      (Class|MediaPlayer|SelectTrack (Variables|MediaPlayer|GetMediaPlayer) "Video" 1)
      (if _returnvalue
        (Default|AddLogText (Variables|Default|GetMainHUD_Ref) (Utilities|Text|FormatText "{name} selected!" (.displayname (Utilities|Array|Get(acopy) (Variables|Devices|GetConnectedCameras) (Variables|Devices|GetConnectedCameraId)))) "(R=1.000000,G=0.750000,B=0.000000,A=1.000000)")
        (else
          (Default|AddLogText (Variables|Default|GetMainHUD_Ref) "Failed to connect to the webcam." "(R=1.000000,G=0.000000,B=0.173601,A=1.000000)")))
      (Variables|Devices|SetConnectedCameraId (Math|Integer|%(Integer) (+ (Variables|Devices|GetConnectedCameraId) 1) (Utilities|Array|Length (Variables|Devices|GetConnectedCameras)))))
    (:then_1
      (Utilities|FlowControl|Delay 2.0)
      (Variables|MediaPlayer|SetWidth (Class|MediaTexture|GetWidth (Variables|MediaPlayer|GetMediaPlayerTexture)))
      (Variables|MediaPlayer|SetHeight (Class|MediaTexture|GetHeight (Variables|MediaPlayer|GetMediaPlayerTexture)))
      ;;[0.9341 1 0] Initialize Texture Render Target
      (bind _returnvalue_2 (Rendering|CreateRenderTarget2D (Variables|MediaPlayer|GetWidth) (Variables|MediaPlayer|GetHeight) "RTF_RGBA8_SRGB"))
      (Variables|MediaPlayer|SetTextureRender _returnvalue_2)
      (Default|AddLogText (Variables|Default|GetMainHUD_Ref) (Utilities|Text|FormatText "Width: {w} Height : {h}" (Variables|MediaPlayer|GetWidth) (Variables|MediaPlayer|GetHeight)) "(R=0.383787,G=1.000000,B=0.000000,A=1.000000)"))))

(event Custom|GetTextureRender
  ;[0 1 0.7159] Refresh Texture Render for capturing live playing
  (bind (_canvas _size _context) (Rendering|BeginDrawCanvastoRenderTarget (Variables|MediaPlayer|GetTextureRender)))
  (Utilities|IsValid _canvas
    (:Is%20Valid
      (Canvas|DrawTexture :self _canvas :RenderTexture "/Game/AlterEgo/Movies/MediaPlayer_Video.MediaPlayer_Video" :ScreenSize (Math|Vector2D|MakeVector2D (Math|Conversions|ToFloat(Integer) (Variables|MediaPlayer|GetWidth)) (Math|Conversions|ToFloat(Integer) (Variables|MediaPlayer|GetHeight))) :CoordinateSize "(X=1.000000,Y=1.000000)" :PivotPoint "(X=0.500000,Y=0.500000)")
      (Rendering|EndDrawCanvastoRenderTarget _context)
      (bind _returnvalue (Class|KismetRenderingLibrary|ReadRenderTargetRawPixelArea (Variables|MediaPlayer|GetTextureRender) 0 0 (Variables|MediaPlayer|GetWidth) (Variables|MediaPlayer|GetHeight) false))
      (Variables|Default|SetPixels _returnvalue))))

(event EventBeginPlay
  (bind _self self)
  (Utilities|FlowControl|Sequence
    (:then_0
      ;[1 1 1] Widget
      (bind _returnvalue (UserInterface|CreateWidget "/Game/AlterEgo/HUD/BPW_MainHUD.BPW_MainHUD_C"))
      (bind _output_get (Variables|Default|SetMainHUD_Ref _returnvalue))
      (UserInterface|Viewport|AddtoViewport _output_get 0)
      (bind _returnvalue_2 (UserInterface|CreateWidget "/Game/AlterEgo/HUD/W_ControlPanel.W_ControlPanel_C" (Game|GetPlayerController 0)))
      (Variables|Default|SetControlPanel_Ref _returnvalue_2)
      (Variables|/Script/Engine.PlayerController|SetbShowMouseCursor _self true)
      (Input|SetInputModeGameandUI _self (Variables|Default|GetMainHUD_Ref) "DoNotLock" true)
      (Default|AddLogText (Variables|Default|GetMainHUD_Ref) "Please wait..." "(R=1.000000,G=1.000000,B=1.000000,A=1.000000)"))
    (:then_1
      (CallFunction|GraphicSetting)
      (CallFunction|GetAllCameras)
      (CallFunction|RetrySpawnCells))))

(event EventTick
  (params (DeltaSeconds :type Float%20%28single-precision%29))
  (CallFunction|GetTextureRender))

(event Input|AxisEvents|InputAxisVertical
  (params (AxisValue :type Float%20%28single-precision%29))
  ;[1 0 0.0186] Control
  (Transformation|AddActorLocalOffset (Game|Player|GetPlayerPawn 0) (Math|Vector|MakeVector (* AxisValue 2.0) 0.0 0.0) false false))

(event Input|AxisEvents|InputAxisHorizontal
  (params (AxisValue :type Float%20%28single-precision%29))
  ;[1 0 0.0186] Control
  (Transformation|AddActorLocalOffset (Game|Player|GetPlayerPawn 0) (Math|Vector|MakeVector 0.0 (* AxisValue 2.0) 0.0) false false))

(event Input|AxisEvents|InputAxisHeight
  (params (AxisValue :type Float%20%28single-precision%29))
  ;[1 0 0.0186] Control
  (Transformation|AddActorLocalOffset (Game|Player|GetPlayerPawn 0) (Math|Vector|MakeVector 0.0 0.0 (* AxisValue 2.0)) false false))

(event Input|KeyboardEvents|N
  (params (Key :type Key%20Structure))
  ;[1 0 0.07694] Load Next Mesh
  (:Pressed
    (CallFunction|LoadNextMeshSells)))

(event Input|KeyboardEvents|1
  (params (Key :type Key%20Structure))
  ;[1 0 0.0186] Quality
  (:Pressed
    (Development|ExecuteConsoleCommand "r.ScreenPercentage = 200" 0)
    (Default|AddLogText (Variables|Default|GetMainHUD_Ref) "Video Quality: Max" "(R=0.000000,G=1.000000,B=0.152926,A=1.000000)")))

(event Input|KeyboardEvents|PageUp
  (params (Key :type Key%20Structure))
  ;[1 0 0.3111] Zoom
  (:Pressed
    (Default|Zoom (.AsBPC%20Alter%20Ego (Utilities|Casting|CastToBPC_AlterEgo (Pawn|GetControlledPawn))) false)))

(event Input|KeyboardEvents|G
  (params (Key :type Key%20Structure))
  ;[1 0 0.09597] Toggle Cell Mode
  (:Pressed
    (CallFunction|ToggleMode)))

(event Input|KeyboardEvents|Tab
  (params (Key :type Key%20Structure))
  (bind _controlpanel_ref (Variables|Default|GetControlPanel_Ref))
  ;[1 0 0.03631] Control Panel
  (:Pressed
    (Utilities|FlowControl|FlipFlop
      (:A
        (Default|PreAddtoViewport _controlpanel_ref)
        (UserInterface|Viewport|AddtoViewport _controlpanel_ref 0))
      (:B
        (Widget|RemovefromParent _controlpanel_ref)))))

(event Input|KeyboardEvents|2
  (params (Key :type Key%20Structure))
  ;[1 0 0.0186] Quality
  (:Pressed
    (Development|ExecuteConsoleCommand "r.ScreenPercentage = 100" 0)
    (Default|AddLogText (Variables|Default|GetMainHUD_Ref) "Video Quality: High" "(R=0.054098,G=1.000000,B=0.000000,A=1.000000)")))

(event Input|KeyboardEvents|3
  (params (Key :type Key%20Structure))
  ;[1 0 0.0186] Quality
  (:Pressed
    (Development|ExecuteConsoleCommand "r.ScreenPercentage = 50" 0)
    (Default|AddLogText (Variables|Default|GetMainHUD_Ref) "Video Quality: Medium" "(R=0.000000,G=1.000000,B=0.152926,A=1.000000)")))

(event Input|KeyboardEvents|4
  (params (Key :type Key%20Structure))
  ;[1 0 0.0186] Quality
  (:Pressed
    (Development|ExecuteConsoleCommand "r.ScreenPercentage = 25" 0)
    (Default|AddLogText (Variables|Default|GetMainHUD_Ref) "Video Quality: Low" "(R=0.000000,G=1.000000,B=0.152926,A=1.000000)")))

(event Input|KeyboardEvents|W
  (params (Key :type Key%20Structure))
  (bind _mainhud_ref (Variables|Default|GetMainHUD_Ref))
  ;[1 0 0.0186] Control
  (:Pressed
    (Utilities|FlowControl|FlipFlop
      (:A
        (Widget|RemovefromParent _mainhud_ref))
      (:B
        (UserInterface|Viewport|AddtoViewport _mainhud_ref 0)))))

(event Input|KeyboardEvents|C
  (params (Key :type Key%20Structure))
  ;[1 0 0.0186] Control
  (:Pressed
    (CallFunction|ConnectDevice)
    (CallFunction|GetTextureRenderandSpawnCells)))

(event Input|KeyboardEvents|S
  (params (Key :type Key%20Structure))
  ;[1 0 0.07983] Increase / Decrease Sell Size
  (:Pressed
    (CallFunction|ScaleSellSize true)))

(event Input|KeyboardEvents|D
  (params (Key :type Key%20Structure))
  ;[1 0 0.07983] Increase / Decrease Sell Size
  (:Pressed
    (CallFunction|ScaleSellSize false)))

(event Input|KeyboardEvents|PageDown
  (params (Key :type Key%20Structure))
  ;[1 0 0.3111] Zoom
  (:Pressed
    (Default|Zoom (.AsBPC%20Alter%20Ego (Utilities|Casting|CastToBPC_AlterEgo (Pawn|GetControlledPawn))) true)))

(fn ConstructionScript)

(fn SpawnCells
  (Utilities|FlowControl|Sequence
    (:then_0
      (bind _outactors (Actor|GetAllActorsOfClass "/Game/AlterEgo/Blueprints/Objects/BP_Cell.BP_Cell_C"))
      (for _array_element _outactors
        (Actor|DestroyActor _array_element)
        (LocalVariables|SetCellScale (/ 0.02 (/ 15.0 (Math|Conversions|ToFloat(Integer) (Variables|Default|GetPixelSize)))))))
    (:then_1
      (while (<= (LocalVariables|GetY) (Variables|MediaPlayer|GetHeight))
        (while (<= (LocalVariables|GetX) (Variables|MediaPlayer|GetWidth))
          (Game|SpawnActorfromClass "/Game/AlterEgo/Blueprints/Objects/BP_Cell.BP_Cell_C" (Math|Transform|MakeTransform (CallFunction|GetCellLocation (LocalVariables|GetX) (LocalVariables|GetY)) "0, 0, 0" (Math|Vector|MakeVector (LocalVariables|GetCellScale) (LocalVariables|GetCellScale) (LocalVariables|GetCellScale))) "Undefined" 0 (Math|Conversions|ToLinearColor(Color) "") (LocalVariables|GetX) (LocalVariables|GetY) "(R=0.000000,G=0.000000,B=0.000000,A=1.000000)" 0)
          (LocalVariables|SetX (+ (LocalVariables|GetX) (Variables|Default|GetPixelSize))))
        (LocalVariables|SetY (+ (LocalVariables|GetY) (Variables|Default|GetPixelSize)))
        (LocalVariables|SetX (Variables|Default|GetPixelSize))))))

(fn GetCellLocation
  (params (X :type Integer) (Y :type Integer))
  (bind _cellsize (LocalVariables|GetCellSize))
  (bind _pixelsize (Variables|Default|GetPixelSize))
  (bind _returnvalue (Math|Conversions|ToFloat(Integer) _pixelsize))
  (bind _returnvalue_2 (/ 15.0 _returnvalue))
  (bind _returnvalue_3 (/ _cellsize _returnvalue_2))
  (return (Math|Vector|MakeVector (/ (- (Math|Conversions|ToFloat(Integer) X) (/ (Math|Conversions|ToFloat(Integer) (Variables|MediaPlayer|GetWidth)) 2.0)) _returnvalue_3) (/ (- (Math|Conversions|ToFloat(Integer) Y) (/ (Math|Conversions|ToFloat(Integer) (Variables|MediaPlayer|GetHeight)) 2.0)) _returnvalue_3) 2.0)))

(fn SpawnSMCells
  (bind _cells (Variables|Default|GetCells))
  (bind _cellscale (LocalVariables|GetCellScale))
  (Utilities|FlowControl|Sequence
    (:then_0
      (bind _outactors (Actor|GetAllActorswithTag "CellGroup"))
      (Variables|Default|SetCellGroup (Utilities|Array|Get(acopy) _outactors))
      (for _array_element _cells
        (Components|DestroyComponent (.Cell (Utilities|Struct|BreakS_Cell _array_element))))
      (Utilities|Array|Clear _cells))
    (:then_1
      (while (<= (LocalVariables|GetY) (Variables|MediaPlayer|GetHeight))
        (while (<= (LocalVariables|GetX) (Variables|MediaPlayer|GetWidth))
          (bind _returnvalue (Class|KismetRenderingLibrary|ReadRenderTargetPixel (Variables|MediaPlayer|GetTextureRender) (LocalVariables|GetX) (LocalVariables|GetY)))
          (bind _returnvalue_2 (AddComponent|AddStaticMeshComponent (Variables|Default|GetCellGroup) false (Math|Transform|MakeTransform (CallFunction|GetCellLocation (LocalVariables|GetX) (LocalVariables|GetY)) "0, 0, 0" (Math|Vector|MakeVector _cellscale _cellscale _cellscale))))
          (bind _output_get (LocalVariables|SetNewCell _returnvalue_2))
          (Components|StaticMesh|SetStaticMesh _output_get "/Engine/BasicShapes/Sphere.Sphere")
          (bind _returnvalue_3 (Rendering|Material|CreateDynamicMaterialInstance (LocalVariables|GetNewCell) 0 "/Game/AlterEgo/Materials/M_Cell.M_Cell" "None" :!class /Script/Engine.PrimitiveComponent))
          (Rendering|Material|SetVectorParameterValue _returnvalue_3 "Color" (Math|Conversions|ToLinearColor(Color) _returnvalue) :!class /Script/Engine.MaterialInstanceDynamic)
          (Utilities|Array|Add (Variables|Default|GetCells) (Utilities|Struct|MakeS_Cell (LocalVariables|GetNewCell) (LocalVariables|GetX) (LocalVariables|GetY) _returnvalue_3))
          (LocalVariables|SetX (+ (LocalVariables|GetX) (LocalVariables|GetCellSize))))
        (LocalVariables|SetY (+ (LocalVariables|GetY) (LocalVariables|GetCellSize)))
        (LocalVariables|SetX (LocalVariables|GetCellSize))))))

(fn GetPixelColor
  (params (X :type Integer) (Y :type Integer))
  (bind _pixels (Variables|Default|GetPixels))
  (bind _width (Variables|MediaPlayer|GetWidth))
  (bind _returnvalue (* Y _width))
  (bind _returnvalue_2 (+ X _returnvalue))
  (bind _output (Utilities|Array|Get(acopy) _pixels _returnvalue_2))
  (if (> (Utilities|Array|Length (Variables|Default|GetPixels)) 0)
    (if (<= (Utilities|Array|Length _pixels) _returnvalue_2)
      _
      (else
        (return (Math|Conversions|ToLinearColor(Color) (Math|Color|MakeColor (Math|Conversions|ToByte(Integer) (Class|KismetMathLibrary|FCeil64 (.b _output))) (Math|Conversions|ToByte(Integer) (Class|KismetMathLibrary|FCeil64 (.g _output))) (Math|Conversions|ToByte(Integer) (Class|KismetMathLibrary|FCeil64 (.r _output))) (Math|Conversions|ToByte(Integer) (Class|KismetMathLibrary|FCeil64 (.a _output)))))))))
  (return ""))

(fn LoadNextMeshSells
  (bind _outactors (Actor|GetAllActorsOfClass "/Game/AlterEgo/Blueprints/Objects/BP_Cell.BP_Cell_C"))
  (for _array_element _outactors
    (Default|LoadNextMesh _array_element)))

(fn ScaleSellSize
  (params (Increase :type Boolean))
  (bind _outactors (Actor|GetAllActorsOfClass "/Game/AlterEgo/Blueprints/Objects/BP_Cell.BP_Cell_C"))
  (for _array_element _outactors
    (Default|ScaleSize _array_element Increase)))

(fn ToggleMode
  (bind _returnvalue (Actor|GetActorOfClass "/Game/AlterEgo/Blueprints/Objects/BP_Cell.BP_Cell_C"))
  (switch Utilities|FlowControl|Switch|SwitchonCellMode (Variables|/Game/AlterEgo/Blueprints/Objects/BP_Cell.BP_Cell_C|GetCellMode _returnvalue)
    (:NewEnumerator0
      (bind _outactors (Actor|GetAllActorsOfClass "/Game/AlterEgo/Blueprints/Objects/BP_Cell.BP_Cell_C"))
      (for _array_element _outactors
        (Default|ChangeMode _array_element "NewEnumerator1"))
      (Development|PrintString "A"))
    (:NewEnumerator1
      (bind _outactors_2 (Actor|GetAllActorsOfClass "/Game/AlterEgo/Blueprints/Objects/BP_Cell.BP_Cell_C"))
      (for _array_element_2 _outactors_2
        (Default|ChangeMode _array_element_2 "NewEnumerator3"))
      (Development|PrintString "B"))
    (:NewEnumerator3
      (bind _outactors_3 (Actor|GetAllActorsOfClass "/Game/AlterEgo/Blueprints/Objects/BP_Cell.BP_Cell_C"))
      (for _array_element_3 _outactors_3
        (Default|ChangeMode _array_element_3 "NewEnumerator0"))
      (Development|PrintString "C"))))

(event Custom|RepaintCells
  (bind _returnvalue (Class|KismetRenderingLibrary|ReadRenderTargetRawPixelArea (Variables|MediaPlayer|GetTextureRender) 0 0 (Variables|MediaPlayer|GetWidth) (Variables|MediaPlayer|GetHeight) false))
  (Variables|Default|SetPixels _returnvalue)
  (for _array_element (Variables|Default|GetCells)
    (Rendering|Material|SetVectorParameterValue (.DynMatIns (Utilities|Struct|BreakS_Cell _array_element)) "Color" (Math|Conversions|ToLinearColor(Color) (Math|Color|MakeColor (Math|Conversions|ToByte(Integer) (Class|KismetMathLibrary|FCeil64 (.b (Utilities|Array|Get(acopy) (Variables|Default|GetPixels) (+ (.X (Utilities|Struct|BreakS_Cell _array_element)) (* (.Y (Utilities|Struct|BreakS_Cell _array_element)) (Variables|MediaPlayer|GetWidth))))))) (Math|Conversions|ToByte(Integer) (Class|KismetMathLibrary|FCeil64 (.g (Utilities|Array|Get(acopy) (Variables|Default|GetPixels) (+ (.X (Utilities|Struct|BreakS_Cell _array_element)) (* (.Y (Utilities|Struct|BreakS_Cell _array_element)) (Variables|MediaPlayer|GetWidth))))))) (Math|Conversions|ToByte(Integer) (Class|KismetMathLibrary|FCeil64 (.r (Utilities|Array|Get(acopy) (Variables|Default|GetPixels) (+ (.X (Utilities|Struct|BreakS_Cell _array_element)) (* (.Y (Utilities|Struct|BreakS_Cell _array_element)) (Variables|MediaPlayer|GetWidth))))))) (Math|Conversions|ToByte(Integer) (Class|KismetMathLibrary|FCeil64 (.a (Utilities|Array|Get(acopy) (Variables|Default|GetPixels) (+ (.X (Utilities|Struct|BreakS_Cell _array_element)) (* (.Y (Utilities|Struct|BreakS_Cell _array_element)) (Variables|MediaPlayer|GetWidth))))))))) :!class /Script/Engine.MaterialInstanceDynamic)))

(event Custom|Test
  (bind _returnvalue (Class|KismetRenderingLibrary|ReadRenderTargetPixel (Variables|MediaPlayer|GetTextureRender) 900 500))
  (Development|PrintString (Utilities|String|Append (Utilities|String|ToString(Byte) (.b _returnvalue)) (Utilities|String|ToString(Byte) (.g _returnvalue)) (Utilities|String|ToString(Byte) (.r _returnvalue)) (Utilities|String|ToString(Byte) (.a _returnvalue))) true true "(R=1.000000,G=0.000000,B=0.923837,A=1.000000)" 5.0)
  (Class|KismetRenderingLibrary|ReadRenderTargetRawPixel (Variables|MediaPlayer|GetTextureRender) 900 500 true)
  (Development|PrintString "Hello" true true "(R=0.000000,G=0.660000,B=1.000000,A=1.000000)" 5.0))
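; BPC_AlterEgo is a base Blueprint for AlterEgo that provides a simple camera zoom.
; Its Zoom function nudges the Camera component's relative Z by a fixed step per call, lowering it when In is true and raising it otherwise, with no limits.
; The event graph and construction script hold no active logic.
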(event EventBeginPlay)

(event Collision|EventActorBeginOverlap
  (params (OtherActor :type Actor%20Object%20Reference)))

(event EventTick
  (params (DeltaSeconds :type Float%20%28single-precision%29)))

(fn ConstructionScript)

(fn Zoom
  (params (In :type Boolean))
  (if In
    (Transformation|SetRelativeLocation (Variables|Default|GetCamera) (Math|Vector|MakeVector 0.0 0.0 (+ (.z (Variables|/Script/Engine.SceneComponent|GetRelativeLocation (Variables|Default|GetCamera))) -2.0)) false false)
    (else
      (Transformation|SetRelativeLocation (Variables|Default|GetCamera) (Math|Vector|MakeVector 0.0 0.0 (+ (.z (Variables|/Script/Engine.SceneComponent|GetRelativeLocation (Variables|Default|GetCamera))) 2.0)) false false))))